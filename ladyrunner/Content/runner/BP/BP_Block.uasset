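; BP_Block is a track segment for a runner game that randomly fills two sidewalk slots and two street lanes with obstacle meshes.
; On BeginPlay it line-traces forward to the neighboring block and blocks a lane's spawn if that block has a truck there.
; Tick slides both street obstacles along world -Y at a fixed per-frame step.
; When BP_Hero overlaps it, the game mode adds a block and this one destroys itself after a delay.
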(event OnComponentBeginOverlap(overlapBox)
  (params (OverlappedComponent :type Primitive%20Component%20Object%20Reference) (OtherActor :type Actor%20Object%20Reference) (OtherComp :type Primitive%20Component%20Object%20Reference) (OtherBodyIndex :type Integer) (bFromSweep :type Boolean) (SweepResult :type Hit%20Result%20Structure%20%28by%20ref%29))
  (Utilities|Casting|CastToBP_Hero OtherActor)
  (Default|AddBlock (Variables|Default|GetGameMode))
  (Utilities|FlowControl|Delay 2.0)
  (Actor|DestroyActor))

(event EventBeginPlay
  (bind _asbp_third_person_game_mode (Utilities|Casting|CastToBP_ThirdPersonGameMode (Game|GetGameMode)))
  (Variables|Default|SetGameMode _asbp_third_person_game_mode)
  (bind _frontblock (CallFunction|CheckFrontBlock))
  (Utilities|IsValid _frontblock
    (:Is%20Valid
      (Variables|Default|SetspawnLane2Car (not (== (Variables|/Script/Engine.StaticMeshComponent|GetStaticMesh (Variables|BP_Block_C|Getobstacle2 _frontblock)) "/Game/AssetsvilleTown/Meshes/Vehicles/SM_veh_truck_merged.SM_veh_truck_merged")))
      (Variables|Default|SetspawnLane3Car (not (== (Variables|/Script/Engine.StaticMeshComponent|GetStaticMesh (Variables|BP_Block_C|Getobstacle3 _frontblock)) "/Game/AssetsvilleTown/Meshes/Vehicles/SM_veh_truck_merged.SM_veh_truck_merged"))))
    (:Is%20Not%20Valid
      _))
  (CallFunction|SpawnObstacles))

(event EventTick
  (params (DeltaSeconds :type Float%20%28single-precision%29))
  (bind _obstacle3 (Variables|Default|Getobstacle3))
  (bind _obstacle2 (Variables|Default|Getobstacle2))
  (Transformation|SetWorldLocation _obstacle2 (+ (Transformation|GetWorldLocation _obstacle2) (* "0.000000,-1.000000,0.000000" 1e+01)) false false)
  (Transformation|SetWorldLocation _obstacle3 (+ (Transformation|GetWorldLocation _obstacle3) (* "0.000000,-1.000000,0.000000" 1e+01)) false false))

(fn ConstructionScript)

(fn SpawnObstacles
  (Utilities|FlowControl|Sequence
    (:then_0
      (if (== (Math|Random|RandomIntegerinRange 0 1) 0)
        (Components|StaticMesh|SetStaticMesh (Variables|Default|Getobstacle1) (Utilities|RandomSidewalkMeshesMacro))))
    (:then_1
      (if (Variables|Default|GetspawnLane2Car)
        (if (== (Math|Random|RandomIntegerinRange 0 1) 0)
          (Components|StaticMesh|SetStaticMesh (Variables|Default|Getobstacle2) (.OutItem (Utilities|Array|Random (Variables|Default|GetStreetMeshes)))))))
    (:then_2
      (if (Variables|Default|GetspawnLane3Car)
        (if (== (Math|Random|RandomIntegerinRange 0 1) 0)
          (Components|StaticMesh|SetStaticMesh (Variables|Default|Getobstacle3) (.OutItem (Utilities|Array|Random (Variables|Default|GetStreetMeshes)))))))
    (:then_3
      (if (== (Math|Random|RandomIntegerinRange 0 1) 0)
        (Components|StaticMesh|SetStaticMesh (Variables|Default|Getobstacle4) (Utilities|RandomSidewalkMeshesMacro))))))

(fn CheckFrontBlock
  (bind _returnvalue (Transformation|GetActorLocation))
  (bind _returnvalue_2 (Transformation|GetActorForwardVector))
  (bind _returnvalue_3 (+ _returnvalue "0.000000,0.000000,20.000000"))
  (bind _outhit (Collision|LineTraceByChannel _returnvalue_3 (+ _returnvalue_3 (* (Math|Vector|MakeVector (.x _returnvalue_2) (.y _returnvalue_2) (+ (.z _returnvalue_2) 0.0)) 1.4e+03)) "TraceTypeQuery1" false 0 "None"))
  (bind _asbp_block (Utilities|Casting|CastToBP_Block (.HitActor (Collision|BreakHitResult _outhit))))
  (return _asbp_block))